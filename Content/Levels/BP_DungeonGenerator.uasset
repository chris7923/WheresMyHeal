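; Dungeon generator Blueprint that calls Generate on BeginPlay and supplies the rules for procedural room and door selection.
; It always starts with RD_1DoorRoom, then picks random NormalRooms until the graph reaches MinNbRoom, after which it returns EndingRoom at door index 0.
; Continue and validity checks always return true, so no stop condition or validation is applied here.
; Every connection uses BP_RegularDoor.
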(event EventBeginPlay
  (PCG|Generate))

(event EventInitializeDungeon
  (params (Rooms :type Dungeon%20Graph%20Object%20Reference)))

(fn ConstructionScript)

(fn ChooseFirstRoomData
  (return "/Game/Levels/RD_1DoorRoom.RD_1DoorRoom"))

(fn ChooseNextRoomData
  (params (CurrentRoom :type Room%20Data%20Object%20Reference) (DoorData :type Door%20Def%20Structure%20%28by%20ref%29))
  (if (>= (Class|DungeonGraph|Count (Variables|Default|GetGraph)) (Variables|Default|GetMinNbRoom))
    (return 0 (Variables|Default|GetEndingRoom))
    (else
      (bind _returnvalue (Class|DungeonGenerator|GetRandomRoomData (Variables|Default|GetNormalRooms)))
      (return -1 _returnvalue))))

(fn ContinuetoAddRoom
  (return true))

(fn IsValidDungeon
  (return true))

(fn ChooseDoor
  (params (CurrentRoom :type Room%20Data%20Object%20Reference) (NextRoom :type Room%20Data%20Object%20Reference) (DoorType :type Door%20Type%20Object%20Reference))
  (if (and (Utilities|IsValid CurrentRoom) (Utilities|IsValid NextRoom))
    (return "/Game/Blueprints/Doors/BP_RegularDoor.BP_RegularDoor_C")
    (else
      (return "/Game/Blueprints/Doors/BP_RegularDoor.BP_RegularDoor_C"))))