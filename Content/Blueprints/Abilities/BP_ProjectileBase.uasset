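; Base projectile ability Blueprint for a pooled ability system, launched along the player character's forward direction.
; ActivateAbility enables physics and collision on the Capsule, then calls LaunchAbility with a fixed-strength vector from player 0's facing.
; LaunchAbility applies it as a velocity-change impulse and prints a debug message.
; PoolAbility only calls its parent, as its nodes for disabling physics and collision are disconnected.
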(event Custom|LaunchAbility
  (params (ImpulseDirection :type Vector))
  (Physics|AddImpulse (Variables|Default|GetCapsule) ImpulseDirection "None" true)
  (Development|PrintString "Launched"))

(event EventBeginPlay
  (|CallParentFunction))

(fn ConstructionScript
  (|CallParentFunction))

(fn PoolAbility
  (|CallParentFunction))

(fn UseAbility
  (|CallParentFunction))

(fn ActivateAbility
  (bind _capsule (Variables|Default|GetCapsule))
  (|CallParentFunction)
  (Physics|SetSimulatePhysics _capsule true)
  (Collision|SetCollisionEnabled _capsule "QueryAndPhysics")
  (CallFunction|LaunchAbility (* (Transformation|GetActorForwardVector (Game|GetPlayerCharacter 0)) (Math|Float|MakeLiteralFloat 1e+03))))