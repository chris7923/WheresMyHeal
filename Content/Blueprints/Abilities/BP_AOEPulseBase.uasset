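; BP_AOEPulseBase is a base area-of-effect pulse ability that applies a buff-type effect to nearby actors.
; UseAbility runs a stationary multi-sphere object trace at the actor's location, filtered to one object type.
; It passes each hit actor, its character status component and the BuffType to ApplyAbilityEffect, then activates the particle system.
; ActivateAbility only calls its parent, and the event graph is unused.
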(event EventBeginPlay
  (|CallParentFunction) ; This node is disabled and will not be called.\nDrag off pins to build functionality.
)

(event Collision|EventActorBeginOverlap
  (params (OtherActor :type Actor%20Object%20Reference)))

(event EventTick
  (params (DeltaSeconds :type Float%20%28single-precision%29)))

(fn ConstructionScript
  (|CallParentFunction))

(fn ActivateAbility
  (|CallParentFunction))

(fn UseAbility
  (bind _returnvalue (Transformation|GetActorLocation))
  (|CallParentFunction)
  (bind _outhits (Collision|MultiSphereTraceForObjects _returnvalue _returnvalue 375.0 (Utilities|Array|MakeArray "ObjectTypeQuery8") false 0 "None" true "(R=1.000000,G=0.000000,B=0.000000,A=1.000000)" "(R=0.000000,G=1.000000,B=0.000000,A=1.000000)" 2.0))
  (for _array_element _outhits
    (CallFunction|ApplyAbilityEffect (.HitActor (Collision|BreakHitResult _array_element)) (Actor|GetComponentbyClass (.HitActor (Collision|BreakHitResult _array_element)) "/Game/Blueprints/Systems/BPC_CharacterStatusComponent.BPC_CharacterStatusComponent_C") (Variables|Default|GetBuffType)))
  (Components|Activation|Activate (Variables|Default|GetParticleSystem) true))