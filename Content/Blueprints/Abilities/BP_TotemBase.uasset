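; Base totem ability actor that periodically applies a buff effect to objects caught in a sphere trace around it.
; UseAbility makes it opaque and plays a grow-and-spin timeline, which starts the looping pulse timer with particles.
; PoolAbility stops pulsing and reverses the timeline, destroying the actor rather than calling parent pooling.
; ActivateAbility shows a half-transparent preview, but the timer driving cursor-aimed GhostPlacement around the player is disconnected.
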(event Custom|TotemPulse
  (bind _totemtick (Variables|Default|GetTotemTick))
  (bind _returnvalue (Utilities|Time|SetTimerbyFunctionName 0 "TotemOverlap" _totemtick true (* _totemtick -1.0)))
  (Variables|Default|SetTotemTimer _returnvalue))

(event Custom|SpawnTotem
  (bind (_direction _lerp _rotaton) (Timeline|GrowTotem PlayFromStart)
    (:Update
      (Transformation|SetActorScale3D (Math|Vector|Lerp(Vector) "0, 0, 0" "1.000000,1.000000,1.000000" _lerp))
      (Transformation|SetActorRotation (Math|Rotator|Lerp(Rotator) "0, 0, 0" "0.000000,359.000000,0.000000" _rotaton)))
    (:Finished
      (switch Utilities|FlowControl|Switch|SwitchonETimelineDirection _direction
        (:Forward
          (CallFunction|TotemPulse))
        (:Backward
          (Actor|DestroyActor))))))

(event Custom|DeleteTotem
  (bind (_direction _lerp _rotaton) (Timeline|GrowTotem ReverseFromEnd)
    (:Update
      (Transformation|SetActorScale3D (Math|Vector|Lerp(Vector) "0, 0, 0" "1.000000,1.000000,1.000000" _lerp))
      (Transformation|SetActorRotation (Math|Rotator|Lerp(Rotator) "0, 0, 0" "0.000000,359.000000,0.000000" _rotaton)))
    (:Finished
      (switch Utilities|FlowControl|Switch|SwitchonETimelineDirection _direction
        (:Forward
          (CallFunction|TotemPulse))
        (:Backward
          (Actor|DestroyActor))))))

(event EventBeginPlay
  (|CallParentFunction))

(event Collision|EventActorBeginOverlap
  (params (OtherActor :type Actor%20Object%20Reference)))

(event EventTick
  (params (DeltaSeconds :type Float%20%28single-precision%29)))

(fn ConstructionScript
  (bind _basemesh (Variables|Default|GetBaseMesh))
  (|CallParentFunction)
  (bind _returnvalue (Rendering|Material|CreateDynamicMaterialInstance _basemesh 0 (Rendering|Material|GetMaterial _basemesh 0) "None" :!class /Script/Engine.PrimitiveComponent))
  (Rendering|Material|SetVectorParameterValue _returnvalue "ColorMultiply" (Variables|Default|GetTESTCOLOR%28DELETELATER%29) :!class /Script/Engine.MaterialInstanceDynamic))

(fn UseAbility
  (|CallParentFunction)
  (CallFunction|SpawnTotem)
  (Utilities|Time|ClearandInvalidateTimerbyHandle (Variables|Default|GetPlacementTimer))
  (Rendering|Material|SetScalarParameterValueonMaterials (Variables|Default|GetBaseMesh) "Opacity" 1.0))

(fn ActivateAbility
  (|CallParentFunction)
  (bind _returnvalue (Rendering|Material|CreateDynamicMaterialInstance (Variables|Default|GetBaseMesh) 0 0 "None" :!class /Script/Engine.PrimitiveComponent))
  (Rendering|Material|SetScalarParameterValue _returnvalue "Opacity" 0.5 :!class /Script/Engine.MaterialInstanceDynamic))

(fn PoolAbility
  (Utilities|Time|ClearandInvalidateTimerbyHandle (Variables|Default|GetTotemTimer))
  (CallFunction|DeleteTotem))

(fn GhostPlacement
  (bind _returnvalue (Game|GetPlayerController 0))
  (bind _returnvalue_2 (Game|GetPlayerCharacter 0))
  (bind _array (Utilities|Array|MakeArray "ObjectTypeQuery9"))
  (bind _hitresult (Class|PlayerController|GetHitResultUnderCursorforObjects _returnvalue _array true))
  (bind _returnvalue_3 (Transformation|GetActorLocation _returnvalue_2))
  (bind _location (Collision|BreakHitResult _hitresult))
  (bind _returnvalue_4 (Math|Rotator|FindLookatRotation _returnvalue_3 _location))
  (bind _returnvalue_5 (Math|Vector|GetForwardVector (Math|Rotator|MakeRotator 0.0 0.0 (.yaw _returnvalue_4))))
  (bind _returnvalue_6 (* _returnvalue_5 3e+02))
  (bind _returnvalue_7 (+ _returnvalue_3 _returnvalue_6))
  (Transformation|SetActorLocation (Math|Vector|MakeVector (.x _returnvalue_7) (.y _returnvalue_7) 0.0) false false))

(fn TotemOverlap
  (bind _returnvalue (Transformation|GetActorLocation))
  (bind _outhits (Collision|MultiSphereTraceForObjects _returnvalue _returnvalue 3e+02 (Utilities|Array|MakeArray "ObjectTypeQuery8") false 0 "None" true "(R=1.000000,G=0.000000,B=0.000000,A=1.000000)" "(R=0.000000,G=1.000000,B=0.000000,A=1.000000)" 0.7))
  (for _array_element _outhits
    (CallFunction|ApplyAbilityEffect (.HitActor (Collision|BreakHitResult _array_element)) (Actor|GetComponentbyClass (.HitActor (Collision|BreakHitResult _array_element)) "/Game/Blueprints/Systems/BPC_CharacterStatusComponent.BPC_CharacterStatusComponent_C") (Variables|Default|GetBuffType)))
  (Components|Activation|Activate (Variables|Default|GetParticleSystem) true))