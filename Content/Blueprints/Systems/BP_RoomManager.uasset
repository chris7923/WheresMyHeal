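; Room encounter manager that locks the party in with enemies until all are killed.
; At BeginPlay it collects doors overlapping its Box and reads party size from the game instance.
; When enough Player or Ally actors enter a non-starting room, it shuts the doors and spawns skeleton warriors at random spawn points if the room is spawnable.
; EnemyKilled counts deaths, then plays brief slow motion and reopens the doors.
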(event OnComponentBeginOverlap(Box)
  (params (OverlappedComponent :type Primitive%20Component%20Object%20Reference) (OtherActor :type Actor%20Object%20Reference) (OtherComp :type Primitive%20Component%20Object%20Reference) (OtherBodyIndex :type Integer) (bFromSweep :type Boolean) (SweepResult :type Hit%20Result%20Structure%20%28by%20ref%29))
  (bind _partymembersinroom (Variables|Default|GetPartyMembersInRoom))
  (if (Math|Boolean|ANDBoolean (not (Variables|Default|GetStartingRoom)) (or (Actor|ActorHasTag OtherActor "Player") (Actor|ActorHasTag OtherActor "Ally")) (not (Variables|Default|GetRoomCleared?)) (not (Variables|Default|GetRoomActive)))
    (Math|Integer|IncrementInt _partymembersinroom
      (:%20%20
        (if (>= _partymembersinroom (Variables|Default|GetMaxPartySize))
          (for _array_element (Variables|Default|GetDoors)
            (Class|Door|Open _array_element false))
          (Variables|Default|SetRoomActive true)
          (CallFunction|SpawnEnemies))))))

(event OnComponentEndOverlap(Box)
  (params (OverlappedComponent :type Primitive%20Component%20Object%20Reference) (OtherActor :type Actor%20Object%20Reference) (OtherComp :type Primitive%20Component%20Object%20Reference) (OtherBodyIndex :type Integer))
  (if (Math|Boolean|ANDBoolean (not (Variables|Default|GetStartingRoom)) (or (Actor|ActorHasTag OtherActor "Player") (Actor|ActorHasTag OtherActor "Ally")) (not (Variables|Default|GetRoomCleared?)))
    (Math|Integer|DecrementInt (Variables|Default|GetPartyMembersInRoom))))

(event Custom|SpawnEnemies
  (bind _spawnpoints (Variables|Default|GetSpawnPoints))
  (bind _returnvalue (Utilities|Array|Length _spawnpoints))
  (bind _returnvalue_2 (Math|Random|RandomInteger _returnvalue))
  (bind _output (Utilities|Array|Get(acopy) _spawnpoints _returnvalue_2))
  (if (Variables|Default|GetSpawnableRoom)
    (for _index (range 1 (Variables|Default|GetMaxEnemiesToSpawn))
      (Game|SpawnActorfromClass "/Game/Blueprints/Characters/AllyAI/BP_AIBaseCharacter.BP_AIBaseCharacter_C" (Math|Transform|MakeTransform (Transformation|GetActorLocation _output) "0, 0, 0" "1.000000,1.000000,1.000000") "AdjustIfPossibleButAlwaysSpawn" "MultiplyWithRoot" 0 self "Enemy" "SkeletonWarrior" "NewEnumerator5" 0)
      (Utilities|Array|RemoveItem (Variables|Default|GetSpawnPoints) _output))))

(event Custom|EnemyKilled
  (bind _enemieskilled (Variables|Default|GetEnemiesKilled))
  (Math|Integer|IncrementInt _enemieskilled
    (:%20%20
      (if (>= _enemieskilled (Variables|Default|GetMaxEnemiesToSpawn))
        (Utilities|Time|SetGlobalTimeDilation 0.3)
        (Utilities|FlowControl|Delay 0.25)
        (Utilities|Time|SetGlobalTimeDilation 1.0)
        (for _array_element (Variables|Default|GetDoors)
          (Class|Door|Open _array_element true))
        (Development|PrintString "Doors opened")
        (Variables|Default|SetRoomCleared? true)))))

(event EventBeginPlay
  (bind _box (Variables|Default|GetBox))
  (bind _partysize (Class|BPIInstanceEvents|GetPartySize(Message) (Game|GetGameInstance)))
  (Variables|Default|SetMaxPartySize _partysize)
  (Collision|SetCollisionEnabled _box "QueryAndPhysics")
  (for _array_element (Collision|GetOverlappingActors _box "/Script/ProceduralDungeon.Door" :!class /Script/Engine.PrimitiveComponent)
    (bind _asdoor (Utilities|Casting|CastToDoor _array_element))
    (Utilities|Array|Add (Variables|Default|GetDoors) _asdoor)))

(fn ConstructionScript)

(fn BasicAttack
  (return 0.0))