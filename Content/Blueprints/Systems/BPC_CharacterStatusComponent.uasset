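; Character status component that tracks health, death and temporary attack speed and damage buffs for its owner.
; Owner damage and timer-driven DOT ticks reduce clamped health, report damage events and update the health widget; heals raise it.
; At zero health, AI owners send kill messages and stop their brain logic, while other owners lose input.
; Heals and buffs spawn Niagara effects, buffs reset after retriggerable delays, and low-health AI allies print a prototype heal plea.
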(event Custom|ChatMessage
  (bind _returnvalue (Components|GetOwner))
  ;[0 1 0.4844] Chat message prototype
  (if (Math|Boolean|ANDBoolean (Utilities|DoesObjectImplementInterface _returnvalue "/Game/Blueprints/Interfaces/BPI_AiInterface.BPI_AiInterface_C") (Actor|ActorHasTag _returnvalue "Ally") (<= (Variables|Default|GetHealth) (* (Variables|Default|GetMaxHealth) 0.45)))
    (Development|PrintString "HEAL ME WTFFFFFF!!!!!!!!!!!!!!!!!!!!!!!!" true true "(R=1.000000,G=0.321990,B=0.000000,A=1.000000)" 2e+01)))

(event Custom|AnyDamage
  (params (DamagedActor :type Actor%20Object%20Reference) (Damage :type Float%20%28single-precision%29) (DamageType :type Damage%20Type%20Object%20Reference) (InstigatedBy :type Controller%20Object%20Reference) (DamageCauser :type Actor%20Object%20Reference))
  (bind _returnvalue (Components|GetOwner))
  (bind _widgetref (Variables|Default|GetWidgetRef))
  (bind _returnvalue_2 (AI|GetAIController _returnvalue))
  ;[0.6641 0 1] Damage Event
  (Variables|Default|SetHealth (Math|Float|Clamp(Float) (- (Variables|Default|GetHealth) Damage) 0.0 (Variables|Default|GetMaxHealth)))
  (Class|AISenseDamage|ReportDamageEvent DamagedActor DamageCauser Damage "0, 0, 0" "0, 0, 0" "None")
  (Utilities|IsValid _widgetref
    (:Is%20Valid
      (Class|BPIUpdateUI|UpdateHealth(Message) (UserInterface|GetWidget _widgetref) (/ (Variables|Default|GetHealth) (Variables|Default|GetMaxHealth)))
      (if (<= (Variables|Default|GetHealth) 0.0)
        (if (Utilities|DoesObjectImplementInterface _returnvalue "/Game/Blueprints/Interfaces/BPI_AiInterface.BPI_AiInterface_C")
          (Utilities|FlowControl|DoOnce false
            (:Completed
              (Variables|Default|SetIsDead true)
              (Class|BPIAiInterface|IsKilled(Message) _returnvalue)
              (Class|BPIAiInterface|GotKill(Message) DamageCauser)
              (Utilities|IsValid _returnvalue_2
                (:Is%20Valid
                  (AI|Logic|StopLogic (Variables|/Script/AIModule.AIController|GetBrainComponent _returnvalue_2) "Dead")))))
          (else
            (Input|DisableInput _returnvalue (Game|GetPlayerController 0))
            (Variables|Default|SetIsDead true)
            (Utilities|FlowControl|Delay 3.0)))
        (else
          (CallFunction|ChatMessage))))))

(event Custom|DOTDamage
  ;[0 1 0.2031] DOT Damage
  (CallFunction|AnyDamage (Components|GetOwner) (stale Custom|StartDOT Damage) 0 0 (stale Custom|StartDOT DamageCauser)))

(event Custom|StartDOT
  (params (Damage :type Float%20%28double-precision%29) (DecayTime :type Float%20%28double-precision%29) (DamageCauser :type Actor%20Object%20Reference))
  ;[0 1 0.2031] DOT Damage
  (bind _returnvalue (Utilities|Time|SetTimerbyEvent (delegate Custom|DOTDamage) 1.0 true -0.8))
  (Utilities|FlowControl|RetriggerableDelay DecayTime)
  (Utilities|Time|ClearandInvalidateTimerbyHandle _returnvalue))

(event EventBeginPlay
  (bind _returnvalue (Components|GetOwner))
  ;[0.007812 1 0] Bind Any Damage Event
  (EventDispatchers|BindEventtoOnTakeAnyDamage _returnvalue (delegate Custom|AnyDamage))
  (Variables|Default|SetWidgetRef (Actor|GetComponentbyClass _returnvalue "/Script/UMG.WidgetComponent")))

(event EventAnyHeal
  (params (HealAmount :type Float%20%28double-precision%29))
  (bind _widgetref (Variables|Default|GetWidgetRef))
  ;[0 0.1328 1] Heal Event
  (bind _output_get (Variables|Default|SetHealth (Math|Float|Clamp(Float) (+ (Variables|Default|GetHealth) HealAmount) 0.0 (Variables|Default|GetMaxHealth))))
  (Niagara|SpawnSystemAttached "/Game/RPGEffects/ParticlesNiagara/Priest/HealBurst/NS_Priest_SimpleHeal.NS_Priest_SimpleHeal" (Variables|/Script/Engine.Actor|GetRootComponent (Components|GetOwner)) "None" "0.000000,0.000000,-50.000000" "0, 0, 0" "SnapToTarget" false true "AutoRelease")
  (Utilities|IsValid _widgetref
    (:Is%20Valid
      (Class|BPIUpdateUI|UpdateHealth(Message) (UserInterface|GetWidget _widgetref) (/ _output_get (Variables|Default|GetMaxHealth))))))

(event EventAnyAttackDamage
  (params (AttackDamage :type Float%20%28double-precision%29))
  (Variables|Default|SetCurrentAttackDamage (+ (Variables|Default|GetCurrentAttackDamage) AttackDamage))
  (Niagara|SpawnSystemAttached "/Game/RPGEffects/ParticlesNiagara/Priest/HealBurst/NS_AttackDamageBuff.NS_AttackDamageBuff" (Variables|/Script/Engine.Actor|GetRootComponent (Components|GetOwner)) "None" "0.000000,0.000000,-50.000000" "0, 0, 0" "KeepRelativeOffset" false)
  (Utilities|FlowControl|RetriggerableDelay 1.9)
  (Variables|Default|SetCurrentAttackDamage (Variables|Default|GetBaseAttackDamage)))

(event EventAnyAttackSpeed
  (params (AttackSpeed :type Float%20%28double-precision%29))
  (bind _output_get (Variables|Default|SetCurrentAttackSpeed (Math|Float|Clamp(Float) (+ (Variables|Default|GetCurrentAttackSpeed) AttackSpeed) 0.3 5.0)))
  (Variables|Default|SetAttackCooldown (/ 1.0 _output_get))
  (Niagara|SpawnSystemAttached "/Game/RPGEffects/ParticlesNiagara/Priest/HealBurst/NS_AttackSpeedBuff.NS_AttackSpeedBuff" (Variables|/Script/Engine.Actor|GetRootComponent (Components|GetOwner)) "None" "0.000000,0.000000,-50.000000" "0, 0, 0" "KeepRelativeOffset" false)
  (Utilities|FlowControl|RetriggerableDelay 1.9)
  (Variables|Default|SetCurrentAttackSpeed (Variables|Default|GetBaseAttackSpeed))
  (Variables|Default|SetAttackCooldown 1.0))

(fn IsDead?
  (return (Variables|Default|GetIsDead)))