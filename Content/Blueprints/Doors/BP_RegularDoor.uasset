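; BP_RegularDoor is a hinged door that calls Open on BeginPlay and animates in response to open and close events.
; The DoorAnimation timeline plays forward to open and in reverse to close, lerping the Hinge's relative rotation through a 110-degree swing.
; When the timeline finishes, its direction decides DoorCollision: disabled after opening, query and physics after closing.
; Lock and unlock events are empty.
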(event EventBeginPlay
  (Class|Door|Open true))

(event Collision|EventActorBeginOverlap
  (params (OtherActor :type Actor%20Object%20Reference)))

(event EventTick
  (params (DeltaSeconds :type Float%20%28single-precision%29)))

(event EventOnDoorOpenBP
  (bind _doorcollision (Variables|Default|GetDoorCollision))
  (bind (_direction _doorlerp) (Timeline|DoorAnimation PlayFromStart)
    (:Update
      (Transformation|SetRelativeRotation (Variables|Default|GetHinge) (Math|Rotator|Lerp(Rotator) "0, 0, 0" "0.000000,-110.000000,0.000000" _doorlerp) false false))
    (:Finished
      (switch Utilities|FlowControl|Switch|SwitchonETimelineDirection _direction
        (:Forward
          (Collision|SetCollisionEnabled _doorcollision "NoCollision"))
        (:Backward
          (Collision|SetCollisionEnabled _doorcollision "QueryAndPhysics"))))))

(event EventOnDoorCloseBP
  (bind _doorcollision (Variables|Default|GetDoorCollision))
  (bind (_direction _doorlerp) (Timeline|DoorAnimation ReverseFromEnd)
    (:Update
      (Transformation|SetRelativeRotation (Variables|Default|GetHinge) (Math|Rotator|Lerp(Rotator) "0, 0, 0" "0.000000,-110.000000,0.000000" _doorlerp) false false))
    (:Finished
      (switch Utilities|FlowControl|Switch|SwitchonETimelineDirection _direction
        (:Forward
          (Collision|SetCollisionEnabled _doorcollision "NoCollision"))
        (:Backward
          (Collision|SetCollisionEnabled _doorcollision "QueryAndPhysics"))))))

(event EventOnDoorLockBP)

(event EventOnDoorUnlockBP)

(fn ConstructionScript)