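; GI_WMHInstance is a game instance Blueprint that stores the party size and hands out usernames.
; An event sets PartySize and a getter function returns it.
; GetUsername picks a random entry from ListOfNames and removes it before returning it, so names are not reused while the instance lives.
; The file shows no refill of the list or handling for when it runs empty.
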(event EventSetPartySize
  (params (PartySize :type Integer))
  (Variables|Default|SetPartySize PartySize))

(fn GetPartySize
  (return (Variables|Default|GetPartySize)))

(fn GetUsername
  (bind _listofnames (Variables|Default|GetListOfNames))
  (bind _output_get (Variables|Default|SetCurrentname (.OutItem (Utilities|Array|Random _listofnames))))
  (Utilities|Array|RemoveItem _listofnames _output_get)
  (return (Variables|Default|GetCurrentname)))