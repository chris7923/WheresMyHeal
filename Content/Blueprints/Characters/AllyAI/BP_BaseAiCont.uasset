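; Base AI controller for combat characters on either the ally or enemy side, driving target acquisition through perception and the blackboard.
; A one-time selection event runs the supplied behavior tree and enables sight and damage senses on the perception component matching the Opponent setting.
; Perception updates fill an empty AttackTarget with living, opponent-tagged actors, clearing it for dead ones.
; SetRange writes and prints attack range; BasicAttack is a stub returning zero.
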(event OnTargetPerceptionUpdated(Enemyperception)
  (params (Actor :type Actor%20Object%20Reference) (Stimulus :type AI%20Stimulus%20Structure))
  (if (== (AI|Components|Blackboard|GetValueasObject (AI|GetBlackboard 0) (Utilities|Name|MakeLiteralName "AttackTarget")) 0)
    (Utilities|SetTarget Actor)))

(event OnTargetPerceptionUpdated(AllyPerception)
  (params (Actor :type Actor%20Object%20Reference) (Stimulus :type AI%20Stimulus%20Structure))
  (if (== (AI|Components|Blackboard|GetValueasObject (AI|GetBlackboard 0) (Utilities|Name|MakeLiteralName "AttackTarget")) 0)
    (Utilities|SetTarget Actor)))

(event Custom|BehaviourTreeSelection
  (params (BTAsset :type Behavior%20Tree%20Object%20Reference))
  (bind _allyperception (Variables|Default|GetAllyPerception))
  (bind _enemyperception (Variables|Default|GetEnemyperception))
  (Utilities|FlowControl|DoOnce false
    (:Completed
      (AI|RunBehaviorTree BTAsset)
      (switch name (Variables|Default|GetOpponent)
        (:Ally
          (Class|AIPerceptionComponent|SetSenseEnabled _enemyperception "/Script/AIModule.AISense_Sight" true)
          (Class|AIPerceptionComponent|SetSenseEnabled _enemyperception "/Script/AIModule.AISense_Damage" true))
        (:Enemy
          (Class|AIPerceptionComponent|SetSenseEnabled _allyperception "/Script/AIModule.AISense_Sight" true)
          (Class|AIPerceptionComponent|SetSenseEnabled _allyperception "/Script/AIModule.AISense_Damage" true))))))

(event Custom|SetRange
  (params (AttackRange :type Float%20%28double-precision%29))
  (bind _returnvalue (AI|GetBlackboard 0))
  (bind _returnvalue_2 (Utilities|Name|MakeLiteralName "AttackRange"))
  (AI|Components|Blackboard|SetValueasFloat _returnvalue _returnvalue_2 AttackRange)
  (Development|PrintString (Utilities|String|ToString(Float) (Class|BlackboardComponent|GetValueasFloat _returnvalue _returnvalue_2)) true true "(R=0.280457,G=0.000000,B=1.000000,A=1.000000)"))

(fn ConstructionScript)

(fn BasicAttack
  (return 0.0))