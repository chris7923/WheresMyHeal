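; Base AI character shared by allies and enemies, configured by team and name at BeginPlay.
; Team data tables supply stats, mesh and attack montage, while BP_BaseAiCont receives the behavior tree, opponent and range; enemies also play a spawn montage.
; Basic attacks box-trace for damage, and abilities spawn actors by cast type (GrabFromPool does no pooling).
; Kills trigger a sphere-trace retarget; death notifies the spawner, then destroys the actor after a delay.
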(event Custom|SpawnAnimation
  (bind _charactermovement (Variables|Character|GetCharacterMovement))
  (Variables|/Script/Engine.CharacterMovementComponent|SetMaxWalkSpeed _charactermovement 0.0)
  (bind _returnvalue (Animation|PlayAnimMontage "/Game/Assets/Animations/SkeletonAnims/AM_SpawnSkeleton.AM_SpawnSkeleton" 1.0 "None"))
  (Utilities|FlowControl|Delay _returnvalue)
  (Variables|/Script/Engine.CharacterMovementComponent|SetMaxWalkSpeed _charactermovement 4e+02))

(event EventBeginPlay
  (Components|SkinnedMesh|HideBonebyName (Variables|Character|GetMesh) "handslot_l" "PBO_None")
  (CallFunction|InitializeAICharacter (Variables|Default|GetTeam) (Utilities|String|StringToName (Utilities|String|EnumtoString (Variables|Default|GetNameSelector)))))

(event EventGotKill
  (bind _returnvalue (Transformation|GetActorLocation))
  (AI|Components|Blackboard|ClearValue (AI|GetBlackboard (Pawn|GetController)) (Utilities|Name|MakeLiteralName "AttackTarget"))
  (bind (_outhits _returnvalue_2) (Collision|MultiSphereTraceForObjects _returnvalue _returnvalue 1.5e+03 (Utilities|Array|MakeArray "ObjectTypeQuery10") false 0 "None"))
  (if _returnvalue_2
    (for _array_element _outhits
      (bind _isdead_ (Class|BPICharacterStatus|IsDead?(Message) (Actor|GetComponentbyClass (.HitActor (Collision|BreakHitResult _array_element)) "/Game/Blueprints/Systems/BPC_CharacterStatusComponent.BPC_CharacterStatusComponent_C")))
      (if (not _isdead_)
        (AI|Components|Blackboard|SetValueasObject (AI|GetBlackboard (Pawn|GetController)) (Utilities|Name|MakeLiteralName "AttackTarget") (.HitActor (Collision|BreakHitResult _array_element)))
        (Development|PrintString (Utilities|GetDisplayName (.HitActor (Collision|BreakHitResult _array_element))))))))

(event EventIsKilled
  (bind _spawnerref (Variables|Default|GetSpawnerRef))
  (Utilities|IsValid _spawnerref
    (:Is%20Valid
      (Default|EnemyKilled _spawnerref))
    (:Is%20Not%20Valid
      _))
  (Collision|SetCollisionEnabled (Variables|Collision|GetCapsuleComponent) "NoCollision")
  (Utilities|FlowControl|Delay 3.0)
  (Actor|DestroyActor))

(event EventBasicAttackHitBox
  (bind _returnvalue (Transformation|GetActorLocation))
  (bind _outhit (Class|KismetSystemLibrary|BoxTraceSingleforObjects _returnvalue (+ _returnvalue (* (Transformation|GetActorForwardVector) (Variables|/Game/Blueprints/Systems/BPC_CharacterStatusComponent.BPC_CharacterStatusComponent_C|GetAttackRange (Variables|Default|GetBPC_DamageComponent)))) "20.000000,20.000000,20.000000" "0, 0, 0" (Utilities|Array|MakeArray (Variables|Default|GetOpponent)) false 0 "ForDuration" true))
  (bind _returnvalue_2 (Game|Damage|ApplyDamage (.HitActor (Collision|BreakHitResult _outhit)) (Variables|/Game/Blueprints/Systems/BPC_CharacterStatusComponent.BPC_CharacterStatusComponent_C|GetCurrentAttackDamage (Variables|Default|GetBPC_DamageComponent)) 0 self))
  (Development|PrintString (Utilities|String|ToString(Float) _returnvalue_2)))

(fn ConstructionScript)

(fn GrabfromPool
  (params (Class :type ABP%20Base%20Ability%20Class%20Reference) (Spawn%20Transform%20Location :type Vector) (Spawn%20Transform%20Scale :type Vector :default "1.000000,1.000000,1.000000"))
  (bind _returnvalue (Game|SpawnActorfromClass :Class Class :SpawnTransform (Math|Transform|MakeTransform Spawn%20Transform%20Location "0, 0, 0" Spawn%20Transform%20Scale) :CollisionHandlingOverride "AlwaysSpawn" :TransformScaleMethod "MultiplyWithRoot" :Instigator 0))
  (Variables|Default|SetCurrentAbility _returnvalue)
  (Default|ActivateAbility _returnvalue))

(fn InitializeAICharacter
  (params (Team :type Name) (RowName :type Name))
  (switch name Team
    (:Ally
      (bind _returnvalue (Utilities|GetDataTableRow "/Game/Blueprints/Data/DT_AllyCharacters.DT_AllyCharacters" RowName)
        (:then
          (bind _attackrange (Utilities|SetValues _returnvalue))
          (bind _asbp_base_ai_cont (Utilities|Casting|CastToBP_BaseAiCont (AI|GetAIController (Pawn|GetController))))
          (Variables|/Game/Blueprints/Characters/AllyAI/BP_BaseAiCont.BP_BaseAiCont_C|SetOpponent _asbp_base_ai_cont "Enemy")
          (Default|BehaviourTreeSelection _asbp_base_ai_cont "/Game/Blueprints/Characters/AllyAI/BT_Ally.BT_Ally")
          (Default|SetRange _asbp_base_ai_cont _attackrange)
          (AI|Components|Blackboard|SetValueasObject (AI|GetBlackboard _asbp_base_ai_cont) (Utilities|Name|MakeLiteralName "Player") (Game|GetPlayerCharacter 0))
          (Variables|Default|SetOpponent "ObjectTypeQuery10"))))
    (:Enemy
      (bind _returnvalue_2 (Utilities|GetDataTableRow "/Game/Blueprints/Data/DT_EnemyCharacters.DT_EnemyCharacters" RowName)
        (:then
          (bind _attackrange_2 (Utilities|SetValues _returnvalue_2))
          (CallFunction|SpawnAnimation)
          (bind _asbp_base_ai_cont_2 (Utilities|Casting|CastToBP_BaseAiCont (AI|GetAIController (Pawn|GetController))))
          (Variables|/Game/Blueprints/Characters/AllyAI/BP_BaseAiCont.BP_BaseAiCont_C|SetOpponent _asbp_base_ai_cont_2 "Ally")
          (Default|BehaviourTreeSelection _asbp_base_ai_cont_2 "/Game/Blueprints/Characters/AllyAI/BT_EasyEnemy.BT_EasyEnemy")
          (Default|SetRange _asbp_base_ai_cont_2 _attackrange_2)
          (Variables|Default|SetOpponent "ObjectTypeQuery8"))))))

(fn AbilityCastType
  (params (CastType :type Enum_CastType%20Enum :default "NewEnumerator4"))
  (switch Utilities|FlowControl|Switch|SwitchonEnum_CastType CastType
    (:NewEnumerator4
      (LocalVariables|SetActorHit self))
    (:NewEnumerator0
      (LocalVariables|SetTargetLocation (+ (Transformation|GetActorLocation) (* (Transformation|GetActorForwardVector) 1e+02))))
    (:NewEnumerator3
      (LocalVariables|SetActorHit (.HitActor (Collision|BreakHitResult (.HitResult (Class|PlayerController|GetHitResultUnderCursorforObjects (Game|GetPlayerController 0) (Utilities|Array|MakeArray "ObjectTypeQuery8") true))))))
    (:NewEnumerator2
      (LocalVariables|SetTargetLocation (.Location (Collision|BreakHitResult (.HitResult (Class|PlayerController|GetHitResultUnderCursorforObjects (Game|GetPlayerController 0) (Utilities|Array|MakeArray "ObjectTypeQuery9") true))))))
    (:NewEnumerator1
      (LocalVariables|SetTargetLocation (+ (Transformation|GetActorLocation) "0.000000,0.000000,200.000000"))))
  (return (LocalVariables|GetTargetLocation) (LocalVariables|GetActorHit)))

(fn CastAbility
  (params (AbilityIndex :type Integer))
  (bind _abilities (Variables|Default|GetAbilities))
  (bind _output (Utilities|Array|Get(acopy) _abilities AbilityIndex))
  (bind (_canuseability _abilityvalues _cooldown _cost _animation _casttype) (Utilities|Struct|BreakS_AbilityData _output))
  (bind (_canuseability_2 _abilityvalues_2 _cooldown_2 _cost_2 _animation_2 _casttype_2 _ability) (Utilities|Struct|BreakS_AbilityData _output))
  (if (Variables|Default|GetCanUseAbility?)
    (if _canuseability
      (Variables|Default|SetCanUseAbility? false)
      (Utilities|Array|SetArrayElem _abilities AbilityIndex (Utilities|SetAbilityActive _output false))
      (Animation|PlayAnimMontage _animation 1.0 "None")
      (bind _target_location (CallFunction|AbilityCastType _casttype))
      (CallFunction|GrabfromPool _ability _target_location "1.000000,1.000000,1.000000")
      (return _cooldown_2 AbilityIndex _output))))

(fn GetHealth
  (return 0.0 0.0))

(fn BasicAttackAnimation
  (bind _bpc_damagecomponent (Variables|Default|GetBPC_DamageComponent))
  (Animation|PlayAnimMontage (Variables|Default|GetBasicAttack) (Variables|/Game/Blueprints/Systems/BPC_CharacterStatusComponent.BPC_CharacterStatusComponent_C|GetCurrentAttackSpeed _bpc_damagecomponent) "None")
  (return (Variables|/Game/Blueprints/Systems/BPC_CharacterStatusComponent.BPC_CharacterStatusComponent_C|GetAttackCooldown _bpc_damagecomponent)))